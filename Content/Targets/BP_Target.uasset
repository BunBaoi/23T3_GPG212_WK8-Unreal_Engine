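; BP_Target is a shootable target that awards the player a point when hit by a first-person projectile.
; On BeginPlay it caches a reference to the first-person character.
; When a BP_FirstPersonProjectile overlaps its Body, it increments that character's Points, destroys itself and plays a sound at its location.
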(event `self.ReceiveBeginPlay`
  (bind _asbp_first_person_character (cast `/Game/FirstPerson/Blueprints/BP_FirstPersonCharacter` (`GameplayStatics.GetPlayerCharacter` 0)))
  (set `self.Chara_Ref` _asbp_first_person_character))

(event `self.Body.OnComponentBeginOverlap`
  (params (OverlappedComponent :type "PrimitiveComponent Object Reference") (OtherActor :type "Actor Object Reference") (OtherComp :type "PrimitiveComponent Object Reference") (OtherBodyIndex :type Integer) (bFromSweep :type Boolean) (SweepResult :type "HitResult Structure (by ref)"))
  (bind _chara_ref (`self.Chara_Ref`))
  (cast `/Game/FirstPerson/Blueprints/BP_FirstPersonProjectile` OtherActor)
  (set `/Game/FirstPerson/Blueprints/BP_FirstPersonCharacter.Points` (+ (`/Game/FirstPerson/Blueprints/BP_FirstPersonCharacter.Points` _chara_ref) 1) _chara_ref)
  (`self.K2_DestroyActor`)
  (`GameplayStatics.PlaySoundAtLocation` "/Game/Targets/SFX-Discord.SFX-Discord" (`self.K2_GetActorLocation`) (struct) 1.0 1.0 0.0 null null null null))

(fn `UserConstructionScript`)